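; BP_NSCollision is an animation notify state that switches on a BP_Character's CapsuleCollision for a window within an animation.
; On notify begin it casts the mesh owner to BP_Character and sets that capsule to query-only collision.
; On notify end it sets the capsule back to no collision, so the notify's span on the timeline defines when it is active.
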(fn `Received_NotifyBegin`
  (params (MeshComp :type "SkeletalMeshComponent Object Reference") (Animation :type "AnimSequenceBase Object Reference") (TotalDuration :type "Float (double-precision)"))
  (returns (ReturnValue :type Boolean))
  (bind (_asbp_character _bsuccess) (cast `/Game/InsideUnreal/Blueprints/BP_Character` (`ActorComponent.GetOwner` MeshComp) :!pure true))
  (if _bsuccess
    (`PrimitiveComponent.SetCollisionEnabled` (`/Game/InsideUnreal/Blueprints/BP_Character.Capsule Collision` _asbp_character) "QueryOnly")
    (return false)))

(fn `Received_NotifyEnd`
  (params (MeshComp :type "SkeletalMeshComponent Object Reference") (Animation :type "AnimSequenceBase Object Reference"))
  (returns (ReturnValue :type Boolean))
  (bind (_asbp_character _bsuccess) (cast `/Game/InsideUnreal/Blueprints/BP_Character` (`ActorComponent.GetOwner` MeshComp) :!pure true))
  (if _bsuccess
    (`PrimitiveComponent.SetCollisionEnabled` (`/Game/InsideUnreal/Blueprints/BP_Character.Capsule Collision` _asbp_character) "NoCollision")
    (return false)))