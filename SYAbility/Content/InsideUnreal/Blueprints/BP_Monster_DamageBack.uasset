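; BP_Monster_DamageBack is a monster Blueprint that reacts to being damaged by a SYCharacter, apparently to strike back at the attacker.
; On BeginPlay it calls the parent, then binds a handler to OnDamaged.
; The DamageBack event sends itself a Health.Damage gameplay event, with itself as Instigator and the attacker as Target.
; A direct BP_GE_BaseAttack effect application is left unconnected.
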(event `self.ReceiveBeginPlay`
  (`parent.ReceiveBeginPlay`)
  (add `self.OnDamaged` (delegate `DamageBack`)))

(event `DamageBack` :!signature `self.OnDamaged`
  (params (DamageAmount :type Integer) (DamageCauser :type "Actor Object Reference"))
  (bind _assycharacter (cast `SYCharacter` DamageCauser))
  (`AbilitySystemBlueprintLibrary.SendGameplayEventToActor` self (struct :`TagName` "Health.Damage") (make `GameplayEventData` (struct) self _assycharacter)))

(event `self.ReceiveTick`
  (params (DeltaSeconds :type "Float (single-precision)")))

(fn `UserConstructionScript`)