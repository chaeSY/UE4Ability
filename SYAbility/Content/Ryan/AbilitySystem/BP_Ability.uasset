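; BP_Ability is an ability Blueprint in Ryan's ability system that handles the casting step, with the cast effect still a placeholder.
; On BeginPlay it gets the HUD from BP_RyanGameMode and begins casting immediately.
; If AbilityDetails has a positive cast time, it shows a HUD cast bar and binds an event to its success.
; Otherwise it calls CastAbility directly, which only prints a debug string.
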(event `self.ReceiveBeginPlay`
  (bind _asbp_ryan_game_mode (cast `/Game/Ryan/BP_RyanGameMode` (`GameplayStatics.GetGameMode`)))
  (set `self.HUD` (`/Game/Ryan/BP_RyanGameMode.HUD` _asbp_ryan_game_mode))
  (`self.BeginCasting`))

(fn `BeginCasting`
  (bind (_abilitydetails_name _abilitydetails_description _abilitydetails_cost _abilitydetails_cooldown _abilitydetails_casttime) (break `/Game/Ryan/AbilitySystem/AbilityDetailsStruct` (`self.AbilityDetails`)))
  (if (> _abilitydetails_casttime 0.0)
    (bind _castbar (`/Game/Ryan/AbilitySystem/UI/WP_HUD.DisplayCastBar` (`self.HUD`) self))
    (add `/Game/Ryan/AbilitySystem/UI/ActionBar/WP_CastBar.CastSuccessful` _castbar (`|CreateDelegate` :!event `CastAbility`))
    (else
      (`self.CastAbility`))))

(fn `CastAbility`
  (`KismetSystemLibrary.PrintString` "Hello"))

(fn `UserConstructionScript`)